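; Grid manager Blueprint that highlights the grid cell under the player's mouse cursor using debug drawing.
; On BeginPlay a looping timer, paced by InteractionRate, runs the highlight check instead of Tick.
; Each check deprojects the cursor, line traces on Visibility up to InteractionDistance, and converts the hit location to a cell.
; A successful lookup briefly draws that cell with DrawDebugCell.
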(event `self.ReceiveBeginPlay`
  (`KismetSystemLibrary.K2_SetTimerDelegate` (delegate `CheckCellHighlight`) (`self.InteractionRate`) true))

(event `CheckCellHighlight`
  (bind _returnvalue (`GameplayStatics.GetPlayerController` 0))
  (bind (_worldlocation _worlddirection) (`PlayerController.DeprojectMousePositionToWorld` _returnvalue))
  (`/Engine/EditorBlueprintResources/StandardMacros.IsValid` _returnvalue
    (:`Is Valid`
      (bind _outhit (`KismetSystemLibrary.LineTraceSingle` :`Start` _worldlocation :`End` (+ _worldlocation (* _worlddirection (`self.InteractionDistance`))) :`TraceChannel` "TraceTypeQuery1" :`DrawTime` 0.1))
      (bind (_outx _outy _returnvalue_2) (`self.GetCellFromWorldPosition` (`.Location` (`GameplayStatics.BreakHitResult` _outhit))))
      (if _returnvalue_2
        (`self.DrawDebugCell` _outx _outy (struct :`G` 255 :`A` 255) 0.1)))))

(fn `UserConstructionScript`)